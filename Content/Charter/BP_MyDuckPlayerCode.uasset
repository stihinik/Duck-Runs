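; Player character that sprints on a stamina pool, collects food and weapons, and tracks survival time with a saved best.
; BeginPlay creates the HUD and inventory actor, then starts a one-second timer that saves new records until GameOver.
; Shift sprint drains SP by timer; F uses overlapped items, with food restoring SP and respawning randomly, weapons entering inventory.
; C scatters the first slot's item into the world and refreshes the held weapon mesh; mouse wheel zooms.
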(event `self.ReceiveBeginPlay`
  (`|ExecutionSequence`
    (:`then_0`
      (bind _returnvalue (`|CreateWidget` "/Game/UI/Main_Canvas.Main_Canvas_C"))
      (bind _output_get (set `self.Main HUD` _returnvalue))
      (`UserWidget.AddToViewport` _returnvalue 0)
      (`UserWidget.AddToViewport` _output_get 0)
      (`self.SpawnInventary`))
    (:`then_1`
      (`/Game/Charter/HealthStats.Set SP` (`self.HealthStats`) 200.0 (`self.Current SP`))
      (`self.Load Time`)
      (`KismetSystemLibrary.K2_SetTimer` null "Increase Time" 1.0 true))))

(event `Key|MouseScrollUp`
  (params (Key :type "Key Structure"))
  (bind _springarm (`self.SpringArm`))
  ;[1 1 1] Увеличение расстрояние камеры
  (:`Pressed`
    (set `SpringArmComponent.TargetArmLength` (`KismetMathLibrary.FClamp` (- (`SpringArmComponent.TargetArmLength` _springarm) (`self.Camera Speed Arm`)) 150.0 600.0) _springarm)))

(event `Key|MouseScrollDown`
  (params (Key :type "Key Structure"))
  (bind _springarm (`self.SpringArm`))
  ;[1 1 1] Уменьшение расстояние камеры
  (:`Pressed`
    (set `SpringArmComponent.TargetArmLength` (`KismetMathLibrary.FClamp` (+ (`SpringArmComponent.TargetArmLength` _springarm) (`self.Camera Speed Arm`)) 150.0 600.0) _springarm)))

(event `self.PickupCollision.OnComponentBeginOverlap`
  (params (OverlappedComponent :type "PrimitiveComponent Object Reference") (OtherActor :type "Actor Object Reference") (OtherComp :type "PrimitiveComponent Object Reference") (OtherBodyIndex :type Integer) (bFromSweep :type Boolean) (SweepResult :type "HitResult Structure (by ref)"))
  (bind _asbp_world_actor (cast `/Game/Inventory/Blueprints/WorldActors/BP_WorldActor` OtherActor))
  (`KismetArrayLibrary.Array_Add` (`self.Array Items to Pickup`) _asbp_world_actor))

(event `Key|LeftShift`
  (params (Key :type "Key Structure"))
  (:`Pressed`
    (`self.Increase Speed` self))
  (:`Released`
    (`self.Decrease Speed` self)))

(event `self.PickupCollision.OnComponentEndOverlap`
  (params (OverlappedComponent :type "PrimitiveComponent Object Reference") (OtherActor :type "Actor Object Reference") (OtherComp :type "PrimitiveComponent Object Reference") (OtherBodyIndex :type Integer))
  (bind _asbp_world_actor (cast `/Game/Inventory/Blueprints/WorldActors/BP_WorldActor` OtherActor))
  (`KismetArrayLibrary.Array_RemoveItem` (`self.Array Items to Pickup`) _asbp_world_actor))

(event `Key|F`
  (params (Key :type "Key Structure"))
  (bind _output (`|GetArrayItem` (`self.Array Items to Pickup`)))
  (bind _item (`/Game/Inventory/Blueprints/WorldActors/BP_WorldActor.Item` _output))
  (bind (_itemsignature_name _itemsignature_type) (break `/Game/Inventory/Structures/S_ItemSignature` (defaults `/Game/Charter/BP_MyDuckPlayerCode` _item)))
  (:`Pressed`
    (`/Engine/EditorBlueprintResources/StandardMacros.IsValid` _output
      (:`Is Valid`
        (switch `/Game/Inventory/Enums/E_ItemType` _itemsignature_type
          (:`NewEnumerator1`
            (`self.Increase SP` self))
          (:`NewEnumerator2`
            (`self.Add Weapon` _item)))
        (`self.Add Item and Create Slot` _output)))))

(event `Key|C`
  (params (Key :type "Key Structure"))
  (bind _item (break `/Game/Inventory/Structures/S_SlotSignature` (`|GetArrayItem` (`/Game/Inventory/Blueprints/BP_Inventary.Slots` (`self.Inventary`)))))
  (:`Pressed`
    (if (`KismetSystemLibrary.IsValidClass` _item)
      (`self. Drop Inventary` _item)
      (`/Game/Inventory/Blueprints/BP_Inventary.Shift Slot` (`self.Inventary`))
      (set `self.AI Run` false)
      (`self.Realod Weapon` (`.item_7_058A200C41C9028C2E12E3B16A2A4C4D` (break `/Game/Inventory/Structures/S_SlotSignature` (`|GetArrayItem` (`/Game/Inventory/Blueprints/BP_Inventary.Slots` (`self.Inventary`))))))
      (`KismetSystemLibrary.PrintString` "предмет в мире")
      (else
        (`KismetSystemLibrary.PrintString` "нет предметов")))))

(fn ` Drop Inventary`
  (params (item :type "/Game/Inventory/Blueprints/ItemClasses/BP_MasterItem_C++ Class Reference"))
  (locals (Knife :type Text :default "NSLOCTEXT(\"\", \"416C21314C30A211CFA18D891FAEDEE7\", \"Knife\")"))
  (bind _itemsignature_name (break `/Game/Inventory/Structures/S_ItemSignature` (defaults `/Game/Charter/BP_MyDuckPlayerCode` item)))
  (bind _out_vector (`self.Random Vector World `))
  (bind _returnvalue (`|SpawnActorFromClass` "/Game/Inventory/Blueprints/WorldActors/BP_WorldActor.BP_WorldActor_C" (`KismetMathLibrary.Conv_VectorToTransform` _out_vector) "AlwaysSpawn" "OverrideRootScale" null item 1 null))
  (bind _item_mesh (`/Game/Inventory/Blueprints/WorldActors/BP_WorldActor.Item Mesh` _returnvalue))
  (`SceneComponent.SetWorldScale3D` _item_mesh (20.0 20.0 20.0))
  (bind _returnvalue_2 (`SceneComponent.K2_GetComponentLocation` _item_mesh))
  (`SceneComponent.K2_SetWorldLocation` _item_mesh (+ _returnvalue_2 (0.0 0.0 50.0)) false false)
  (if (`KismetTextLibrary.EqualEqual_TextText` _itemsignature_name (`local.Knife`))
    (`SceneComponent.K2_SetWorldLocation` _item_mesh (+ _returnvalue_2 (0.0 0.0 100.0)) false false)))

(fn `Add Item and Create Slot`
  (params (Item :type "/Game/Inventory/Blueprints/WorldActors/BP_WorldActor Object Reference"))
  (locals (`local item` :type "/Game/Inventory/Blueprints/WorldActors/BP_WorldActor Object Reference"))
  (bind _output_get (set `local.local item` Item))
  (bind _item (`/Game/Inventory/Blueprints/WorldActors/BP_WorldActor.Item` _output_get))
  (bind (_itemsignature_name _itemsignature_type) (break `/Game/Inventory/Structures/S_ItemSignature` (defaults `/Game/Charter/BP_MyDuckPlayerCode` _item)))
  (switch `/Game/Inventory/Enums/E_ItemType` _itemsignature_type
    (:`NewEnumerator1`
      (`self. Drop Inventary` _item)
      (`self.K2_DestroyActor` (`local.local item`)))
    (:`NewEnumerator2`
      (bind (_success _result) (`/Game/Inventory/Blueprints/BP_Inventary.Add Item` (`self.Inventary`) _item 1))
      (switch `/Game/Inventory/Enums/E_AddItemResult` _result
        (:`NewEnumerator0`
          (`KismetSystemLibrary.PrintString` "Добавлен")
          (`self.K2_DestroyActor` (`local.local item`)))
        (:`NewEnumerator2`
          (`KismetSystemLibrary.PrintString` "Нет места в инвентаре"))))))

(fn `Add Weapon`
  (params (WeaponItem :type "/Game/Inventory/Blueprints/ItemClasses/BP_MasterItem_C++ Class Reference"))
  (locals (LocalNameWeapon :type Text))
  (bind (_itemsignature_name _itemsignature_type _itemsignature_2dicon _itemsignature_3dmesh _itemsignature_airun _itemsignature_stackablecanbestacked _itemsignature_useblecanbeused _itemsignature_typeweapon) (break `/Game/Inventory/Structures/S_ItemSignature` (defaults `/Game/Charter/BP_MyDuckPlayerCode` WeaponItem)))
  (bind _weaponitem (`self.WeaponItem`))
  (bind _weaponitem_2 (`self.WeaponItem`))
  (if (`/Game/Inventory/Blueprints/BP_Inventary.Get Slot Info from Index` (`self.Inventary`) 0)
    (set `self.AI Run` _itemsignature_airun)
    (`StaticMeshComponent.SetStaticMesh` _weaponitem_2 _itemsignature_3dmesh)
    (`SceneComponent.SetWorldScale3D` _weaponitem_2 (5.0 5.0 5.0))
    (switch `/Game/Inventory/Enums/E_TypeWeapon` _itemsignature_typeweapon
      (:`NewEnumerator0`
        (`SceneComponent.K2_SetRelativeLocation` _weaponitem (-26.0 -3.0 -27.0) false false))
      (:`NewEnumerator1`
        (`SceneComponent.K2_SetRelativeLocation` _weaponitem (-33.0 7.0 -8.0) false false)))))

(fn `Decrease SP`
  (bind _returnvalue (- (`self.Current SP`) 2.0))
  (if (<= _returnvalue 0.0)
    (bind _output_get (set `self.Current SP` 0.0))
    (`/Game/Charter/HealthStats.Set SP` (`self.HealthStats`) 200.0 _output_get)
    (`self.Decrease Speed` self)
    (else
      (bind _output_get_2 (set `self.Current SP` _returnvalue))
      (`/Game/Charter/HealthStats.Set SP` (`self.HealthStats`) 200.0 _output_get_2))))

(fn `Decrease Speed`
  (bind _maxwalkspeed (`CharacterMovementComponent.MaxWalkSpeed` (`self.CharacterMovement`)))
  (if (> _maxwalkspeed 200.0)
    (if (>= (`self.Current SP`) 0.0)
      (set `CharacterMovementComponent.MaxWalkSpeed` (- _maxwalkspeed (`self.Run`)) (`self.CharacterMovement`))
      (`KismetSystemLibrary.K2_ClearAndInvalidateTimerHandle` (`self.Close Timer`)))))

(fn `Increase SP`
  (bind _returnvalue (+ (`self.Current SP`) 20.0))
  (bind _output_get (set `self.Current SP` (`KismetMathLibrary.SelectFloat` 200.0 _returnvalue (>= _returnvalue 200.0))))
  (`/Game/Charter/HealthStats.Set SP` (`self.HealthStats`) 200.0 _output_get))

(fn `Increase Speed`
  (if (> (`self.Current SP`) 0.0)
    (set `CharacterMovementComponent.MaxWalkSpeed` (+ (`CharacterMovementComponent.MaxWalkSpeed` (`self.CharacterMovement`)) (`self.Run`)) (`self.CharacterMovement`))
    (bind _returnvalue (`KismetSystemLibrary.K2_SetTimer` null "Decrease SP" 1.0 true))
    (set `self.Close Timer` _returnvalue)))

(fn `Increase Time`
  (bind _max_time (`self.Max Time`))
  (if (not (`self.GameOver`))
    (bind _output_get (set `self.Current Time` (+ (`self.Current Time`) 1)))
    (if (> _output_get _max_time)
      (bind _output_get_2 (set `self.Max Time` (`self.Current Time`)))
      (`/Game/Charter/HealthStats.Set Time` (`self.HealthStats`) _output_get_2 (`self.Max Time`))
      (bind _returnvalue (`GameplayStatics.CreateSaveGameObject` "/Game/General_Blueprint/Save_Time_BP.Save_Time_BP_C"))
      (set `/Game/General_Blueprint/Save_Time_BP.Max Time` (`self.Max Time`) _returnvalue)
      (`GameplayStatics.SaveGameToSlot` _returnvalue "MaxTime")
      (else
        (`/Game/Charter/HealthStats.Set Time` (`self.HealthStats`) _output_get _max_time)))))

(fn `Load Time`
  (bind _returnvalue (`GameplayStatics.DoesSaveGameExist` "MaxTime"))
  (if _returnvalue
    (bind _returnvalue_2 (`GameplayStatics.LoadGameFromSlot` "MaxTime"))
    (bind _assave_time_bp (cast `/Game/General_Blueprint/Save_Time_BP` _returnvalue_2))
    (set `self.Max Time` (`/Game/General_Blueprint/Save_Time_BP.Max Time` _assave_time_bp))
    (`/Game/Charter/HealthStats.Set Time` (`self.HealthStats`) 0 (`self.Max Time`))))

(fn `Random Vector World `
  (returns (`Out Vector` :type "Vector Structure"))
  (locals (Vector :type "Vector Structure"))
  (bind _output_get (set `local.Vector` (`KismetMathLibrary.MakeVector` (`KismetMathLibrary.RandomFloatInRange` -8000.0 3500.0) (`KismetMathLibrary.RandomFloatInRange` -7000.0 6000.0) 220.0)))
  (return _output_get))

(fn `Realod Weapon`
  (params (WeaponItem :type "/Game/Inventory/Blueprints/ItemClasses/BP_MasterItem_C++ Class Reference"))
  (bind (_itemsignature_name _itemsignature_type _itemsignature_2dicon _itemsignature_3dmesh _itemsignature_airun _itemsignature_stackablecanbestacked _itemsignature_useblecanbeused _itemsignature_typeweapon) (break `/Game/Inventory/Structures/S_ItemSignature` (defaults `/Game/Charter/BP_MyDuckPlayerCode` WeaponItem)))
  (bind _weaponitem (`self.WeaponItem`))
  (bind _weaponitem_2 (`self.WeaponItem`))
  (if (not (`/Game/Inventory/Blueprints/BP_Inventary.Get Slot Info from Index` (`self.Inventary`) 0))
    (set `self.AI Run` _itemsignature_airun)
    (`StaticMeshComponent.SetStaticMesh` _weaponitem_2 _itemsignature_3dmesh)
    (`SceneComponent.SetWorldScale3D` _weaponitem_2 (5.0 5.0 5.0))
    (switch `/Game/Inventory/Enums/E_TypeWeapon` _itemsignature_typeweapon
      (:`NewEnumerator0`
        (`SceneComponent.K2_SetRelativeLocation` _weaponitem (-26.0 -3.0 -27.0) false false))
      (:`NewEnumerator1`
        (`SceneComponent.K2_SetRelativeLocation` _weaponitem (-33.0 7.0 -8.0) false false)))
    (else
      (set `self.AI Run` false)
      (`StaticMeshComponent.SetStaticMesh` (`self.WeaponItem`) null))))

(fn `SpawnInventary`
  (bind _returnvalue (`|SpawnActorFromClass` "/Game/Inventory/Blueprints/BP_Inventary.BP_Inventary_C" (`self.GetTransform` self) "Undefined" "OverrideRootScale" null (`self.Inventory Slots Initialization`) (`self.Amounts of Slots Initialization`) self (`self.Main HUD`) null null))
  (set `self.Inventary` _returnvalue)
  (return))

(fn `UserConstructionScript`)