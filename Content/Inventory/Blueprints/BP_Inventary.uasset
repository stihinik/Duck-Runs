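; Inventory Blueprint that stores item class and amount pairs in a fixed-size slot array and displays them on the HUD.
; BeginPlay sizes the array, links itself to the main HUD's inventory widget and generates slot widgets.
; AddItem fills the first empty slot and ShiftSlot moves entries down one index, both regenerating the widgets.
; Stack search and runtime widget creation helpers exist but are not called here.
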(event `self.ReceiveBeginPlay`
  (`KismetArrayLibrary.Array_Resize` (`self.Slots`) (`self.Amount of Slots`))
  (set `/Game/Inventory/Widgets/InventaryWB.BP_Inventary Ref` self (`/Game/UI/Main_Canvas.InventaryWB_199` (`self.Main HUD Ref`)))
  (bind _output_get (set `self.InvWBRef` (`/Game/UI/Main_Canvas.InventaryWB_199` (`self.Main HUD Ref`))))
  (`/Game/Inventory/Widgets/InventaryWB.Generate Slot Widgets` _output_get))

(fn `Add Item`
  (params (Item :type "/Game/Inventory/Blueprints/ItemClasses/BP_MasterItem_C++ Class Reference") (Amounts :type Integer))
  (returns (Success :type Boolean) (Result :type "/Game/Inventory/Enums/E_AddItemResult Enum"))
  (locals (`Local Item ` :type "/Game/Inventory/Blueprints/ItemClasses/BP_MasterItem_C++ Class Reference") (`Local Amount` :type Integer))
  (set `local.Local Item ` Item)
  (bind _output_get (set `local.Local Amount` Amounts))
  (if (> _output_get 0)
    (bind (_success _index) (`self.Search an Empty Slot`))
    (if _success
      (`KismetArrayLibrary.Array_Set` (`self.Slots`) _index (make `/Game/Inventory/Structures/S_SlotSignature` (`local.Local Item `) (`local.Local Amount`)))
      (`self.Update Widjet Slot`)
      (return true "NewEnumerator0")
      (else
        (return false "NewEnumerator2")))))

(fn `Create Inventary Widget`
  (bind (_returnvalue_x _returnvalue_y) (`KismetMathLibrary.BreakVector2D` (`WidgetLayoutLibrary.GetViewportSize`)))
  (bind _returnvalue (`|CreateWidget` "/Game/Inventory/Widgets/InventaryWB.InventaryWB_C" null self))
  (bind _output_get (set `self.InvWBRef` _returnvalue))
  (`Widget.SetVisibility` _output_get "Visible")
  (bind _returnvalue_2 (`CanvasPanel.AddChildToCanvas` (`/Game/UI/Main_Canvas.CanvasPanel_0` (`self.Main HUD Ref`)) _output_get))
  (`CanvasPanelSlot.SetAutoSize` _returnvalue_2 true)
  (`CanvasPanelSlot.SetPosition` _returnvalue_2 (`KismetMathLibrary.MakeVector2D` (* _returnvalue_x 1.0) (* _returnvalue_y 1.0)))
  (return))

(fn `Get Slot Info from Index`
  (params (Index :type Integer))
  (returns (Empty :type Boolean) (ItemSignature :type "/Game/Inventory/Structures/S_ItemSignature Structure") (Amount :type Integer))
  (bind (_item _amount) (break `/Game/Inventory/Structures/S_SlotSignature` (`|GetArrayItem` (`self.Slots`) Index)))
  (if (`KismetSystemLibrary.IsValidClass` _item)
    (return false (defaults `/Game/Inventory/Blueprints/BP_Inventary` _item) _amount)
    (else
      (return true (struct) 0))))

(fn `Search an Empty Slot`
  (returns (Success :type Boolean) (Index :type Integer))
  (locals (`Local Boolean` :type Boolean) (`Local Index` :type Integer))
  (for (_array_element _array_index) (`self.Slots`)
    (if (not (`KismetSystemLibrary.IsValidClass` (`.item_7_058A200C41C9028C2E12E3B16A2A4C4D` (break `/Game/Inventory/Structures/S_SlotSignature` _array_element))))
      (set `local.Local Boolean` true)
      (set `local.Local Index` _array_index)
      (break)))
  (return (`local.Local Boolean`) (`local.Local Index`)))

(fn `Search Slot Index for Stack`
  (params (Item :type "/Game/Inventory/Blueprints/ItemClasses/BP_MasterItem Class Reference"))
  (returns (Success :type Boolean) (`Founded Index` :type Integer))
  (locals (`Local Stack is Founder` :type Boolean))
  (for (_array_element _array_index) (`self.Slots`)
    (bind _item (break `/Game/Inventory/Structures/S_SlotSignature` _array_element))
    (if (and (`KismetSystemLibrary.IsValidClass` _item) (== _item Item))
      (set `local.Local Stack is Founder` true)
      (break)))
  (return (`local.Local Stack is Founder`) _array_index))

(fn `Shift Slot`
  (for (_ _array_index) (`self.Slots`)
    (`KismetArrayLibrary.Array_Set` (`self.Slots`) _array_index (`|GetArrayItem` (`self.Slots`) (+ _array_index 1)))
    (`self.Update Widjet Slot`)))

(fn `Update Widjet Slot`
  (`/Game/Inventory/Widgets/InventaryWB.Generate Slot Widgets` (`self.InvWBRef`)))

(fn `UserConstructionScript`)