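; World actor that displays an inventory item as a rotating 3D mesh.
; Initialize3DMesh reads the 3dMesh from the class defaults of the Item class and assigns it to ItemMesh.
; It runs in both the construction script and BeginPlay.
; Tick adds a fixed local rotation each frame without delta-time scaling, so spin speed depends on frame rate.
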(event `self.ReceiveBeginPlay`
  (`self.Initialize 3D Mesh`))

(event `self.ReceiveTick`
  (params (DeltaSeconds :type "Float (single-precision)"))
  (`self.K2_AddActorLocalRotation` (struct :`Yaw` 2.0)))

(fn `Initialize 3D Mesh`
  (bind (_itemsignature_name _itemsignature_type _itemsignature_2dicon _itemsignature_3dmesh) (break `/Game/Inventory/Structures/S_ItemSignature` (defaults `/Game/Inventory/Blueprints/WorldActors/BP_WorldActor` (`self.Item`))))
  (`StaticMeshComponent.SetStaticMesh` (`self.Item Mesh`) _itemsignature_3dmesh)
  (return))

(fn `UserConstructionScript`
  (`self.Initialize 3D Mesh`))